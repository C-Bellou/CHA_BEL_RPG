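; BP_NPC is an interactable NPC actor with a dialogue camera and speech bubble.
; Interract uses a FlipFlop to show its text render, blend the view to itself and block player movement, then reverse all three.
; Talking increments TalkIndex and shows that Dialogue entry in the TopDown controller's Bubble widget, removing it and resetting once the index exceeds the array length.
; Left click only hides the text render.
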(event `Key|LeftMouseButton`
  (params (Key :type "Key Structure"))
  ; Left click interract with Dialogue
  (:`Pressed`
    (`SceneComponent.SetVisibility` (`self.TextRender1`) false false)))

(event `self.ReceiveBeginPlay`
  ; Left click interract with Dialogue
  (`self.EnableInput` (`GameplayStatics.GetPlayerController` 0)))

(event `self.Interract`
  (bind _player_controller (`/Game/Blueprint/BP_FL_Shortcut.GetTopDownController`))
  (bind _player_controller_2 (`/Game/Blueprint/BP_FL_Shortcut.GetTopDownController`))
  (`/Engine/EditorBlueprintResources/StandardMacros.FlipFlop`
    (:`A`
      (`KismetSystemLibrary.PrintString` "A")
      (`SceneComponent.SetVisibility` (`self.TextRender1`) true false)
      (`PlayerController.SetViewTargetWithBlend` _player_controller_2 self 1.0 "VTBlend_Linear" 1.0 false)
      (set `/Game/TopDown/Blueprints/BP_TopDownController.ShouldMove` false _player_controller_2)
      (`KismetSystemLibrary.PrintString` "NO MOVE"))
    (:`B`
      (`KismetSystemLibrary.PrintString` "B")
      (`SceneComponent.SetVisibility` (`self.TextRender1`) false false)
      (`PlayerController.SetViewTargetWithBlend` _player_controller (`Controller.K2_GetPawn` _player_controller) 1.0 "VTBlend_Linear" 0.0 false)
      (set `/Game/TopDown/Blueprints/BP_TopDownController.ShouldMove` true _player_controller)
      (`KismetSystemLibrary.PrintString` "MOVE"))))

(event `Talking`
  (`SceneComponent.SetVisibility` (`self.TextRender1`) false false)
  (`/Engine/EditorBlueprintResources/StandardMacros.IncrementInt` (`self.TalkIndex`)
    (:`  `
      (if (<= (`self.TalkIndex`) (`KismetArrayLibrary.Array_Length` (`self.Dialogue`)))
        (`UserWidget.AddToViewport` (`/Game/TopDown/Blueprints/BP_TopDownController.Bubble` (`/Game/Blueprint/BP_FL_Shortcut.GetTopDownController`)) 0)
        (`TextBlock.SetText` (`/Game/UI/WBP_Dialogue.TalkText` (`/Game/TopDown/Blueprints/BP_TopDownController.Bubble` (`/Game/Blueprint/BP_FL_Shortcut.GetTopDownController`))) (`KismetTextLibrary.Conv_StringToText` (`|GetArrayItem` (`self.Dialogue`) (`self.TalkIndex`))))
        (else
          (`Widget.RemoveFromParent` (`/Game/TopDown/Blueprints/BP_TopDownController.Bubble` (`/Game/Blueprint/BP_FL_Shortcut.GetTopDownController`)))
          (set `self.TalkIndex` 0))))))

(fn `UserConstructionScript`)