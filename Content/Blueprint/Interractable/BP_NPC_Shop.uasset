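; Interactable NPC shopkeeper actor that opens and closes an in-world shop screen for the player.
; On interaction it blends the top-down controller's camera to itself, shows its widget component, initializes the WBP_Shop with itself and blocks player movement.
; ExitShop hides the widget, restores movement and blends the view back to the controlled pawn.
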(event `self.Interract`
  (bind _widget (`self.Widget`))
  (`PlayerController.SetViewTargetWithBlend` (`/Game/Blueprint/BP_FL_Shortcut.GetTopDownController`) self 1.0 "VTBlend_Linear" 1.0 false)
  (`SceneComponent.SetVisibility` _widget true false)
  (bind _aswbp_shop (cast `/Game/UI/WBP_Shop` (`WidgetComponent.GetWidget` _widget)))
  (`/Game/UI/WBP_Shop.InitializeShop` _aswbp_shop self)
  (`KismetSystemLibrary.PrintString` "NPCS")
  (set `/Game/TopDown/Blueprints/BP_TopDownController.ShouldMove` false (`/Game/Blueprint/BP_FL_Shortcut.GetTopDownController`)))

(event `ExitShop`
  (bind _player_controller (`/Game/Blueprint/BP_FL_Shortcut.GetTopDownController`))
  (`SceneComponent.SetVisibility` (`self.Widget`) false false)
  (`KismetSystemLibrary.PrintString` "should")
  (set `/Game/TopDown/Blueprints/BP_TopDownController.ShouldMove` true (`/Game/Blueprint/BP_FL_Shortcut.GetTopDownController`))
  (`PlayerController.SetViewTargetWithBlend` _player_controller (`Controller.K2_GetPawn` _player_controller) 1.0 "VTBlend_Linear" 0.0 false))

(fn `UserConstructionScript`)